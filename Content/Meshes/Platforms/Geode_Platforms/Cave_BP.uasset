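; Cave_BP is a construction-time builder that lays cave spline mesh sections along its Spline component.
; The construction script derives SectionLength from the actor's Y scale, then BuildCave adds one Y-forward, collision-enabled spline mesh per whole section.
; StartPos receives a clamped tangent instead of the start location, which is left unused, and StartTangent stays unclamped.
; The event graph has no active logic.
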(fn `Build_Cave`
  (bind _spline (`self.Spline`))
  (for _index (range (`KismetMathLibrary.FFloor` (/ (`SplineComponent.GetSplineLength` (`self.Spline`)) (`self.Section_length`))))
    (bind _returnvalue (`AddComponent|NODE_AddSplineMeshComponent-0`))
    (`SplineMeshComponent.SetForwardAxis` _returnvalue "Y" true)
    (`PrimitiveComponent.SetCollisionEnabled` _returnvalue "QueryAndPhysics")
    (bind _returnvalue_2 (`SplineComponent.GetTangentAtDistanceAlongSpline` (`self.Spline`) (* _index (`self.Section_Length`)) "Local"))
    (bind _returnvalue_3 (* (+ _index 1) (`self.Section_Length`)))
    (`SplineMeshComponent.SetStartAndEnd` _returnvalue (`KismetMathLibrary.ClampVectorSize` _returnvalue_2 0.0 (`self.Section_Length`)) _returnvalue_2 (`SplineComponent.GetLocationAtDistanceAlongSpline` _spline _returnvalue_3 "Local") (`KismetMathLibrary.ClampVectorSize` (`SplineComponent.GetTangentAtDistanceAlongSpline` _spline _returnvalue_3 "Local") 0.0 (`self.Section_Length`)) true)))

(fn `UserConstructionScript`
  (bind (_returnvalue_x _returnvalue_y) (`KismetMathLibrary.BreakVector` (`self.GetActorScale3D`)))
  (set `self.Section_Length` (* _returnvalue_y 2852.0))
  (`self.Build_Cave`))