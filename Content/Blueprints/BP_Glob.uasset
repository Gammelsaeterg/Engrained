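; Glob enemy character that AI can order to attack a target and that drops health orbs when killed.
; An attack turns it toward the target on a timeline, then plays a montage.
; A toggleable hitbox with Niagara trails damages one non-Glob actor per activation.
; TakeDamage weakens low-knockback hits; death detaches the controller, replays the death montage if interrupted, and fades dynamic materials before destroying the actor.
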(event `StartDefaultAttackSequence`
  (if (not (`self.bIsAttacking`))
    (set `self.bIsAttacking` true)
    (`self.TurnToTarget`)))

(event `TurnToTarget`
  (set `CharacterMovementComponent.bOrientRotationToMovement` false (`self.CharacterMovement`))
  (set `self.ControllerRotationBeforeTurning` (`SceneComponent.K2_GetComponentRotation` (`self.CapsuleComponent`)))
  (bind _currenttargetactor (`self.CurrentTargetActor`)
    (:`then`
      (set `self.TargetActorLocation` (`self.K2_GetActorLocation` _currenttargetactor))
      (bind (_direction _turncurve) (`Timeline|TurnTowardsTargetTimeline` :!via `PlayFromStart` :!label _label)
        (:`Update`
          (bind (_returnvalue_roll _returnvalue_pitch _returnvalue_yaw) (`KismetMathLibrary.BreakRotator` (`KismetMathLibrary.RLerp` (`self.ControllerRotationBeforeTurning`) (`KismetMathLibrary.Conv_VectorToRotator` (- (`self.TargetActorLocation`) (`self.K2_GetActorLocation` self))) _turncurve true)))
          (`self.K2_SetActorRotation` (`KismetMathLibrary.MakeRotator` 0.0 0.0 _returnvalue_yaw)))
        (:`Finished`
          (set `CharacterMovementComponent.bOrientRotationToMovement` true (`self.CharacterMovement`))
          (`|PlayMontage` (`self.Mesh`) "/Game/Meshes/Glob/GlobAttack_Anim_rig_Glob_Attack__23__Montage.GlobAttack_Anim_rig_Glob_Attack__23__Montage"
            (:`then`
              (set `self.bIsAttacking` true))
            (:`OnCompleted`
              (set `self.bIsAttacking` false :!label _label_2))
            (:`OnInterrupted`
              (goto _label_2))))))
    (:`else`
      (goto _label_2))))

(event `CancelTurn`
  (set `CharacterMovementComponent.bOrientRotationToMovement` true (`self.CharacterMovement`))
  (`|ExecutionSequence`
    (:`then_0`
      (goto _label :!via `Stop`))
    (:`then_1`
      (set `self.bIsAttacking` false))))

(event `/Game/Blueprints/AI/BPI_ActionsAI.AttackAI`
  (`self.StartDefaultAttackSequence`))

(event `ActivateHitbox`
  (`ActorComponent.Activate` (`self.NS_GlobTrails`) true)
  (set `PrimitiveComponent.bGenerateOverlapEvents` true (`self.AttackHitbox`))
  (set `self.bAttackHasHit` false))

(event `/Game/Blueprints/AI/BPI_ActionsAI.AcivateHitbox`
  (params (bAcivate :type Boolean))
  (if bAcivate
    (`self.ActivateHitbox`)
    (else
      (`self.DeactivateHitbox`))))

(event `DeactivateHitbox`
  (`ActorComponent.Deactivate` (`self.NS_GlobTrails`))
  (set `PrimitiveComponent.bGenerateOverlapEvents` false (`self.AttackHitbox`)))

(event `self.AttackHitbox.OnComponentBeginOverlap`
  (params (OverlappedComponent :type "PrimitiveComponent Object Reference") (OtherActor :type "Actor Object Reference") (OtherComp :type "PrimitiveComponent Object Reference") (OtherBodyIndex :type Integer) (bFromSweep :type Boolean) (SweepResult :type "HitResult Structure (by ref)"))
  (bind (_returnvalue_location _returnvalue_rotation) (`KismetMathLibrary.BreakTransform` (`SceneComponent.K2_GetComponentToWorld` (`self.AttackHitbox`))))
  (if (and (not (== OtherActor self)) (not (== (`GameplayStatics.GetObjectClass` OtherActor) "BP_Glob_C")))
    (if (not (`self.bAttackHasHit`))
      (message `/Game/Blueprints/BPI_CombatInteractionInterface.TakeDamage` OtherActor (`SceneComponent.K2_GetComponentLocation` (`self.AttackHitbox`)) (0.0 0.0 0.0) 34.0 0.0)
      (set `self.bAttackHasHit` true)
      (`NiagaraFunctionLibrary.SpawnSystemAtLocation` "/Game/Particles/NS_GlobHit.NS_GlobHit" _returnvalue_location _returnvalue_rotation))))

(event `UndoInterruption`
  (`|PlayMontage` (`self.Mesh`) "/Game/Meshes/Glob/GlobDeath_Anim_rig_Glob_Death__45__Montage.GlobDeath_Anim_rig_Glob_Death__45__Montage" :!label _label_3
    (:`OnCompleted`
      (bind (_direction _fadetrack) (`Timeline|FadeOut` :!via `PlayFromStart` :!label _label_4)
        (:`Update`
          (for _array_element (`self.DynamicMaterials`)
            (`MaterialInstanceDynamic.SetScalarParameterValue` _array_element "FadeOpacity" _fadetrack)))
        (:`Finished`
          (`self.K2_DestroyActor`))))
    (:`OnBlendOut`
      (set `SkeletalMeshComponent.bPauseAnims` true (`self.Mesh`))
      (goto _label_4 :!via `PlayFromStart`))
    (:`OnInterrupted`
      (`self.UndoInterruption`))))

(event `self.ReceiveBeginPlay`
  (`self.SetupDynamicMaterials`))

(event `DefeatSequence`
  (bind (_returnvalue_location _returnvalue_rotation _returnvalue_scale) (`KismetMathLibrary.BreakTransform` (`self.GetTransform`)))
  (set `self.bIsKill` true)
  (`|ExecutionSequence`
    (:`then_0`
      (for _ (range 5)
        (`|SpawnActorFromClass` "/Game/Blueprints/BP_HealthOrb.BP_HealthOrb_C" (`KismetMathLibrary.MakeTransform` (`SceneComponent.K2_GetComponentLocation` (`self.Mesh`)) _returnvalue_rotation _returnvalue_scale) "Undefined" "OverrideRootScale" null 3.0 self)))
    (:`then_1`
      (`self.DetachFromControllerPendingDestroy`)
      (set `PrimitiveComponent.bGenerateOverlapEvents` false (`self.CapsuleComponent`))
      (`PrimitiveComponent.SetCollisionResponseToChannel` (`self.CapsuleComponent`) "ECC_Pawn" "ECR_Ignore")
      (`SkeletalMeshComponent.Stop` (`self.Mesh`))
      (goto _label_3))))

(event `SetupDynamicMaterials`
  (for (_array_element _array_index) (`MeshComponent.GetMaterials` (`self.Mesh`))
    (bind _returnvalue (`PrimitiveComponent.CreateDynamicMaterialInstance` (`self.Mesh`) _array_index _array_element "None"))
    (`KismetArrayLibrary.Array_Add` (`self.DynamicMaterials`) _returnvalue)))

(fn `GetIsAttacking`
  (returns (bIsAttacking :type Boolean))
  (return (`self.bIsAttacking`)))

(fn `SetTargetActor`
  (params (InActor :type "Actor Object Reference"))
  (set `self.CurrentTargetActor` InActor)
  (return))

(fn `TakeDamage`
  (params (HitLocation :type "Vector Structure") (HitDirection :type "Vector Structure") (Damage :type "Float (double-precision)") (KnockbackPower :type "Float (double-precision)"))
  (returns (bHitReceived :type Boolean))
  ;[1 1 1] Take damage
  (if (not (`self.bIsKill`))
    (if (< KnockbackPower 5.0)
      (set `self.HealthPoints` (- (`self.HealthPoints`) (/ Damage 5.0)))
      (else
        (set `self.HealthPoints` (- (`self.HealthPoints`) Damage))))
    (if (< (`self.HealthPoints`) 0.0)
      (`GameplayStatics.SpawnSoundAttached` "/Game/Sounds/Shroob/S_globHurt_death.S_globHurt_death" (`self.Mesh`) "None" (0.0 0.0 0.0) (struct) "KeepRelativeOffset" false 1.0 1.0 0.0 "/Game/Sounds/SA_CaveSoundAttenuation.SA_CaveSoundAttenuation" "/Game/Sounds/SC_DefaultConcurrency.SC_DefaultConcurrency")
      (`self.DefeatSequence`)
      (else
        (`|ExecutionSequence`
          (:`then_0`
            (if (not (`self.bIsKill`))
              (`GameplayStatics.SpawnSoundAttached` "/Game/Sounds/Shroob/S_globHurt.S_globHurt" (`self.AttackHitbox`) "None" (0.0 0.0 0.0) (struct) "KeepRelativeOffset" false 1.0 1.0 0.0 "/Game/Sounds/SA_CaveSoundAttenuation.SA_CaveSoundAttenuation" "/Game/Sounds/SC_DefaultConcurrency.SC_DefaultConcurrency")
              (return true)))
          (:`then_1`
            (return true)))))))

(fn `UserConstructionScript`)