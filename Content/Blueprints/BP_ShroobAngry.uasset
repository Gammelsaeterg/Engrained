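; Flying Shroob enemy that taunts when turned hostile and attacks its target with either a spit projectile or a dive.
; A randomized looping timer picks the attack; the dive lerps the mesh along timeline curves to the target's saved position and back, with a single-hit damage box.
; Hits nudge the mesh and reduce health; death launches a ragdoll, drops health orbs and fades dynamic materials before destroying the actor.
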(event `SetupDynamicMaterials`
  (for (_array_element _array_index) (`MeshComponent.GetMaterials` (`self.VisibleMesh`))
    (bind _returnvalue (`PrimitiveComponent.CreateDynamicMaterialInstance` (`self.VisibleMesh`) _array_index _array_element "None"))
    (`KismetArrayLibrary.Array_Add` (`self.DynamicMaterials`) _returnvalue)))

(event `self.EventHostile`
  (params (Hostile :type Boolean))
  (if Hostile
    (`/Engine/EditorBlueprintResources/StandardMacros.DoOnce` false :!label _label
      (:`Completed`
        (`|ExecutionSequence`
          (:`then_0`
            (set `self.bEnemyDetected` true)
            (`GameplayStatics.SpawnSoundAttached` "/Game/Sounds/Shroob/S_shrobTaunt.S_shrobTaunt" (`self.VisibleMesh`) "None" (0.0 0.0 0.0) (struct) "KeepRelativeOffset" false 1.0 1.0 0.0 "/Game/Sounds/SA_CaveSoundAttenuation.SA_CaveSoundAttenuation" "/Game/Sounds/SC_DefaultConcurrency.SC_DefaultConcurrency"))
          (:`then_1`
            (goto _label_2 :!via `Reset`)))))
    (else
      (`/Engine/EditorBlueprintResources/StandardMacros.DoOnce` false :!label _label_2
        (:`Completed`
          (`|ExecutionSequence`
            (:`then_0`
              (set `self.bEnemyDetected` false))
            (:`then_1`
              (goto _label :!via `Reset`))))))))

(event `self.EventDeath`
  (bind (_returnvalue_location _returnvalue_rotation _returnvalue_scale) (`KismetMathLibrary.BreakTransform` (`self.GetTransform`)))
  (`/Engine/EditorBlueprintResources/StandardMacros.DoOnce` false
    (:`Completed`
      (for _ (range 5)
        (`|SpawnActorFromClass` "/Game/Blueprints/BP_HealthOrb.BP_HealthOrb_C" (`KismetMathLibrary.MakeTransform` (`SceneComponent.K2_GetComponentLocation` (`self.VisibleMesh`)) _returnvalue_rotation _returnvalue_scale) "Undefined" "OverrideRootScale" null 3.0 self)
        (set `self.bIsKill` true)
        (`PrimitiveComponent.SetSimulatePhysics` (`self.VisibleMesh`) true)
        (`PrimitiveComponent.SetCollisionProfileName` (`self.VisibleMesh`) "Ragdoll" false)
        (`PrimitiveComponent.AddImpulse` (`self.VisibleMesh`) (* (`self.LastSavedHitDirection`) 300.0) "None" true)
        (`KismetSystemLibrary.Delay` 0.5)
        (`|SpawnActorFromClass` "/Game/Blueprints/Shroob/BP_PoisonCloud.BP_PoisonCloud_C" (`KismetMathLibrary.MakeTransform` (`SceneComponent.K2_GetComponentLocation` (`self.VisibleMesh`))) "Undefined" "OverrideRootScale" null self)
        (bind (_direction _fadetrack) (`Timeline|FadeOutTimeline`)
          (:`Update`
            (for _array_element (`self.DynamicMaterials`)
              (`MaterialInstanceDynamic.SetScalarParameterValue` _array_element "FadeOpacity" _fadetrack)))
          (:`Finished`
            (`self.K2_DestroyActor`)))))))

(event `SelfDestroyed`
  (set `self.bIsKill` true))

(event `self.ReceiveBeginPlay`
  (`parent.ReceiveBeginPlay`)
  (`self.SetupDynamicMaterials`)
  (`self.SaveOriginalRelativePosition`)
  (`self.UpdateShrobLocation`)
  (`KismetSystemLibrary.K2_SetTimerDelegate` (delegate `AttackTarget`) (`KismetMathLibrary.RandomFloatInRange` 1.5 2.0) true))

(event `self.ReceiveTick`
  (params (DeltaSeconds :type "Float (single-precision)"))
  (`parent.ReceiveTick` DeltaSeconds)
  (`self.TickShroobHit`)
  (if (<= (`self.HealthPoints`) 0.0)
    (`self.Death`)))

(event `TickShroobHit`)

(event `ShrobSpitAttack`
  (bind _returnvalue (`self.GetTargetActor`))
  (`|SpawnActorFromClass` "/Game/Blueprints/BP_ShrobSpit.BP_ShrobSpit_C" (`KismetMathLibrary.MakeTransform` (`SceneComponent.K2_GetComponentLocation` (`self.ProjectileSpawnSocket`)) (`KismetMathLibrary.Conv_VectorToRotator` (`KismetMathLibrary.Normal` (- (`self.K2_GetActorLocation` _returnvalue) (`SceneComponent.K2_GetComponentLocation` (`self.ProjectileSpawnSocket`)))))) "Undefined" "OverrideRootScale" null (`self.ProjectileDamage`) 10.0 500.0 0.0 4.0 self)
  (`GameplayStatics.SpawnSoundAttached` "/Game/Sounds/Shroob/S_shrobprojectile.S_shrobprojectile" (`self.VisibleMesh`) "None" (`self.K2_GetActorLocation`) (struct) "KeepRelativeOffset" false 1.0 1.0 0.0 "/Game/Sounds/SA_CaveSoundAttenuation.SA_CaveSoundAttenuation" "/Game/Sounds/SC_DefaultConcurrency.SC_DefaultConcurrency"))

(event `AttackTarget`
  (if (`self.bEnemyDetected`)
    (if (not (`self.bIsDoingAttack`))
      (if (`KismetMathLibrary.RandomBool`)
        (`self.ShrobDiveAttack`)
        (else
          (`|PlayMontage` (`self.VisibleMesh`) "/Game/Meshes/CrescentShroob/CrescentShrob_flying_spit_adjusted_Montage.CrescentShrob_flying_spit_adjusted_Montage"
            (:`then`
              (set `self.bIsDoingAttack` true))
            (:`OnCompleted`
              (set `self.bIsDoingAttack` false))))))))

(event `CancelAttack`)

(event `SaveOriginalRelativePosition`
  (set `self.OriginalRelativeLocation` (`SceneComponent.RelativeLocation` (`self.VisibleMesh`))))

(event `UpdateShrobLocation`
  (set `self.ShrobLastSavedLocation` (+ (`SceneComponent.K2_GetComponentLocation` (`self.SensingSphere`)) (`self.OriginalRelativeLocation`))))

(event `ShrobDiveAttack`
  (bind _shroblastsavedlocation (`self.ShrobLastSavedLocation`))
  (bind _returnvalue (`self.GetTargetActor`))
  (set `self.bIsDoingAttack` true)
  (set `self.LastSavedActorLocation` (`self.K2_GetActorLocation` _returnvalue))
  (`self.UpdateShrobLocation`)
  (`|PlayMontage` (`self.VisibleMesh`) "/Game/Meshes/CrescentShroob/ShrobDiveAttack_Montage.ShrobDiveAttack_Montage"
    (:`then`
      (`|ExecutionSequence`
        (:`then_0`
          (goto _label_3 :!via `Reset`))
        (:`then_1`
          (bind (_direction _travelcurve _retreatcurve) (`Timeline|DiveAttackTimeline` :!via `PlayFromStart`)
            (:`Update`
              (if (not (`self.bIsKill`))
                (`SceneComponent.K2_SetWorldLocation` (`self.VisibleMesh`) (+ (`KismetMathLibrary.VLerp` _shroblastsavedlocation (`self.LastSavedActorLocation`) _travelcurve) (`KismetMathLibrary.MakeVector` 0.0 0.0 _retreatcurve)) false false)
                (else
                  (`/Engine/EditorBlueprintResources/StandardMacros.DoOnce` false :!label _label_3
                    (:`Completed`
                      (`self.CancelAttack`))))))
            (:`Finished`
              (set `self.bIsDoingAttack` false)
              (if (not (`self.bIsKill`))
                (`SceneComponent.K2_SetWorldLocation` (`self.VisibleMesh`) _shroblastsavedlocation false false)
                (`self.UpdateShrobLocation`)))))))))

(event `StartDiveBox`
  ;[1 1 1] DiveAttack hitbox
  (set `PrimitiveComponent.bGenerateOverlapEvents` true (`self.ShrobDiveAttackBox`))
  (set `self.bDiveAttackHasHit` false))

(event `EndDiveBox`
  ;[1 1 1] DiveAttack hitbox
  (set `PrimitiveComponent.bGenerateOverlapEvents` false (`self.ShrobDiveAttackBox`)))

(event `self.ShrobDiveAttackBox.OnComponentBeginOverlap`
  (params (OverlappedComponent :type "PrimitiveComponent Object Reference") (OtherActor :type "Actor Object Reference") (OtherComp :type "PrimitiveComponent Object Reference") (OtherBodyIndex :type Integer) (bFromSweep :type Boolean) (SweepResult :type "HitResult Structure (by ref)"))
  (bind (_returnvalue_location _returnvalue_rotation) (`KismetMathLibrary.BreakTransform` (`SceneComponent.K2_GetComponentToWorld` (`self.ShrobDiveAttackBox`))))
  ;[1 1 1] DiveAttack hitbox
  (if (and (not (== OtherActor self)) (not (== (`GameplayStatics.GetObjectClass` OtherActor) "BP_ShroobAngry_C")))
    (if (not (`self.bDiveAttackHasHit`))
      (message `/Game/Blueprints/BP_CombatInteractionInterface.TakeDamage` OtherActor (`SceneComponent.K2_GetComponentLocation` (`self.ShrobDiveAttackBox`)) (0.0 0.0 0.0) 21.0 0.0)
      (set `self.bDiveAttackHasHit` true)
      (`NiagaraFunctionLibrary.SpawnSystemAtLocation` "/Game/Particles/NS_ShrobHit.NS_ShrobHit" _returnvalue_location _returnvalue_rotation))))

(fn `TakeDamage`
  (params (HitLocation :type "Vector Structure") (HitDirection :type "Vector Structure") (Damage :type "Float (double-precision)") (KnockbackPower :type "Float (double-precision)"))
  (returns (bHitReceived :type Boolean))
  ;[1 1 1] Take damage
  (if (not (`self.bIsKill`))
    (set `self.HealthPoints` (- (`self.HealthPoints`) Damage))
    (bind _output_get (set `self.LastSavedHitDirection` HitDirection))
    (if (< (`self.HealthPoints`) 0.0)
      (`GameplayStatics.SpawnSoundAttached` "/Game/Sounds/Shroob/S_shrobHurt_death.S_shrobHurt_death" (`self.VisibleMesh`) "None" (0.0 0.0 0.0) (struct) "KeepRelativeOffset" false 1.0 1.0 0.0 "/Game/Sounds/SA_CaveSoundAttenuation.SA_CaveSoundAttenuation" "/Game/Sounds/SC_DefaultConcurrency.SC_DefaultConcurrency")
      (`self.SelfDestroyed`))
    (`KismetSystemLibrary.PrintString` (`KismetStringLibrary.Concat_StrStr` "Damage taken: " (`KismetStringLibrary.Conv_DoubleToString` Damage) " HealthPoits left: " (`KismetStringLibrary.Conv_DoubleToString` (`self.HealthPoints`))))
    (`|ExecutionSequence`
      (:`then_0`
        (if (not (`self.bIsKill`))
          (`SceneComponent.K2_SetRelativeLocation` (`self.VisibleMesh`) (+ (`SceneComponent.RelativeLocation` (`self.VisibleMesh`)) (* _output_get 20.0)) false false)
          (`GameplayStatics.SpawnSoundAttached` "/Game/Sounds/Shroob/S_shrobHurt.S_shrobHurt" (`self.VisibleMesh`) "None" (0.0 0.0 0.0) (struct) "KeepRelativeOffset" false 1.0 1.0 0.0 "/Game/Sounds/SA_CaveSoundAttenuation.SA_CaveSoundAttenuation" "/Game/Sounds/SC_DefaultConcurrency.SC_DefaultConcurrency")
          (return true)))
      (:`then_1`
        (return true)))))

(fn `UserConstructionScript`
  (`parent.UserConstructionScript`))