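; BP_CrescentGameMode is a game mode handling respawn of the player's BP_Mina character.
; BeginPlay and Respawn bind OnDestroyed to the current Mina, but that handler is empty.
; Tick polls IsDestroyed, which nothing here sets true, then after a delay spawns and possesses a new Mina at SpawnTransform, rebinds and clears the flag.
; RespawnPawnsEvent only prints ScenePawns names and saved locations, without respawning them.
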(event `self.RespawnPawnsEvent`
  (`KismetSystemLibrary.PrintString` "Respawning pawns")
  (for (_array_element _array_index) (`self.ScenePawns`)
    (`KismetSystemLibrary.PrintString` (`KismetStringLibrary.Concat_StrStr` "Respawning: " (`KismetSystemLibrary.GetDisplayName` _array_element) " at location: " (`KismetStringLibrary.Conv_VectorToString` (`|GetArrayItem` (`self.ScenePawnsLocations`) _array_index))) true true (struct :`R` 0.279545 :`G` 0.218776 :`B` 0.369792 :`A` 1.0))))

(event `Respawn`
  ;[1 1 1] Respawn System
  (bind _asbp_mina (cast `/Game/Blueprints/Mina/BP_Mina` (`GameplayStatics.GetPlayerCharacter` 0) :!label _label))
  (if true
    (add `Actor.OnDestroyed` _asbp_mina (delegate `On Destroyed`))))

(event `self.ReceiveBeginPlay`
  ;[1 1 1] Respawn System
  (goto _label))

(event `On Destroyed`
  (params (DestroyedActor :type "Actor Object Reference"))
  ;[1 1 1] Respawn System
)

(event `self.ReceiveTick`
  (params (DeltaSeconds :type "Float (single-precision)"))
  ;[1 1 1] Respawn System
  (if (`self.Is Destroyed`)
    (`KismetSystemLibrary.Delay` 1.0)
    (bind _returnvalue (`|SpawnActorFromClass` "/Game/Blueprints/Mina/BP_Mina.BP_Mina_C" (`self.Spawn Transform`) "Undefined" "OverrideRootScale" null null))
    (`Controller.Possess` (`GameplayStatics.GetPlayerController` 0) _returnvalue)
    (`self.Respawn`)
    (set `self.Is Destroyed` false)))

(fn `UserConstructionScript`)