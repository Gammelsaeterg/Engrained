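; BP_PoisonCloud is a short-lived hazard that damages the player's MinaExperimental pawn while it stands inside.
; Its sphere starts hidden and without collision, becomes visible and query-only after a short delay, then the actor destroys itself seconds later.
; Sphere overlaps toggle a damage flag, and Tick sends repeated damage messages through a DoOnce that resets after a brief delay.
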(event `self.ReceiveBeginPlay`
  (bind _sphere (`self.Sphere`))
  (bind _sphere_2 (`self.Sphere`))
  (`PrimitiveComponent.SetCollisionEnabled` _sphere_2 "NoCollision")
  (`SceneComponent.SetVisibility` _sphere_2 false false)
  (bind _asmina_experimental (cast `MinaExperimental` (`GameplayStatics.GetPlayerPawn` 0)))
  (set `self.As Mina Experimental` _asmina_experimental)
  (`KismetSystemLibrary.Delay` 0.75)
  (`PrimitiveComponent.SetCollisionEnabled` _sphere "QueryOnly")
  (`SceneComponent.SetVisibility` _sphere true false)
  (`KismetSystemLibrary.Delay` 5.0)
  (`self.K2_DestroyActor`))

(event `self.ReceiveTick`
  (params (DeltaSeconds :type "Float (single-precision)"))
  (if (`self.bTakeDamage`)
    (`/Engine/EditorBlueprintResources/StandardMacros.DoOnce` false :!label _label
      (:`Completed`
        (message `/Game/Blueprints/BP_CombatInteractionInterface.TakeDamage` (`self.As Mina Experimental`) (0.0 0.0 0.0) (0.0 0.0 0.0) 1.0 0.0)
        (`KismetSystemLibrary.Delay` 0.2)
        (goto _label :!via `Reset`)))))

(event `self.Sphere.OnComponentBeginOverlap`
  (params (OverlappedComponent :type "PrimitiveComponent Object Reference") (OtherActor :type "Actor Object Reference") (OtherComp :type "PrimitiveComponent Object Reference") (OtherBodyIndex :type Integer) (bFromSweep :type Boolean) (SweepResult :type "HitResult Structure (by ref)"))
  (if (== OtherActor (`self.As Mina Experimental`))
    (set `self.bTakeDamage` true)))

(event `self.Sphere.OnComponentEndOverlap`
  (params (OverlappedComponent :type "PrimitiveComponent Object Reference") (OtherActor :type "Actor Object Reference") (OtherComp :type "PrimitiveComponent Object Reference") (OtherBodyIndex :type Integer))
  (if (== OtherActor (`self.As Mina Experimental`))
    (set `self.bTakeDamage` false)))

(fn `UserConstructionScript`)