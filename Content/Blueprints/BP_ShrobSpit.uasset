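; BP_ShrobSpit is a spit projectile Blueprint that adds a wobbling, pulsing look to its ProjectileMesh on top of parent class behavior.
; BeginPlay picks a random frequency per axis, so each instance deforms differently.
; Tick sets relative scale around one using per-axis cosines of game time.
; The cosine is multiplied by delta seconds without accumulating, so wobble amplitude varies with frame rate.
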(event `self.ReceiveBeginPlay`
  (`parent.ReceiveBeginPlay`)
  (set `self.RandomFrequency1` (`KismetMathLibrary.RandomFloatInRange` 3.0 7.0))
  (set `self.RandomFrequency2` (`KismetMathLibrary.RandomFloatInRange` 3.0 7.0))
  (set `self.RandomFrequency3` (`KismetMathLibrary.RandomFloatInRange` 3.0 7.0)))

(event `self.ReceiveTick`
  (params (DeltaSeconds :type "Float (single-precision)"))
  (`SceneComponent.SetRelativeScale3D` (`self.ProjectileMesh`) (`KismetMathLibrary.MakeVector` (+ (* (* (`KismetMathLibrary.Cos` (* (`KismetSystemLibrary.GetGameTimeInSeconds`) (`self.RandomFrequency1`))) 20.0) DeltaSeconds) 1.0) (+ (* (* (`KismetMathLibrary.Cos` (* (`KismetSystemLibrary.GetGameTimeInSeconds`) (`self.RandomFrequency2`))) 20.0) DeltaSeconds) 1.0) (+ (* (* (`KismetMathLibrary.Cos` (* (`KismetSystemLibrary.GetGameTimeInSeconds`) (`self.RandomFrequency3`))) 20.0) DeltaSeconds) 1.0))))

(fn `UserConstructionScript`
  (`parent.UserConstructionScript`))