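; BP_CrystalProjectilePrototype is a prototype projectile actor that damages and knocks back what it hits.
; BeginPlay launches it along the mesh's forward vector at ProjectileSpeed, while a separate Fire event only sets InitialSpeed.
; Mesh overlap with anything except the instigator sends TakeDamageMessage, spawns the NS_BulletHit effect and destroys the projectile.
; A disconnected copy of the impact logic, without damage, never runs.
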(event `Fire`
  (set `ProjectileMovementComponent.InitialSpeed` 300.0 (`self.ProjectileMovement`)))

(event `self.ProjectileMesh.OnComponentBeginOverlap`
  (params (OverlappedComponent :type "PrimitiveComponent Object Reference") (OtherActor :type "Actor Object Reference") (OtherComp :type "PrimitiveComponent Object Reference") (OtherBodyIndex :type Integer) (bFromSweep :type Boolean) (SweepResult :type "HitResult Structure (by ref)"))
  (bind (_returnvalue_location _returnvalue_rotation _returnvalue_scale) (`KismetMathLibrary.BreakTransform` (`self.GetTransform` self)))
  (if (not (== (`self.GetInstigator`) OtherActor))
    (message `/Game/Blueprints/BP_CombatInteractionInterface.TakeDamage` OtherActor _returnvalue_location (`KismetMathLibrary.Normal` (`SceneComponent.GetForwardVector` (`self.ProjectileMesh`))) (`self.ProjectileDamage`) (`self.KnockbackPower`))
    (`NiagaraFunctionLibrary.SpawnSystemAtLocation` "/Game/Particles/NS_BulletHit.NS_BulletHit" _returnvalue_location _returnvalue_rotation _returnvalue_scale)
    (`self.K2_DestroyActor`)))

(event `self.ReceiveBeginPlay`
  (set `MovementComponent.Velocity` (* (`SceneComponent.GetForwardVector` (`self.ProjectileMesh`)) (`self.ProjectileSpeed`)) (`self.ProjectileMovement`)))

(fn `UserConstructionScript`)