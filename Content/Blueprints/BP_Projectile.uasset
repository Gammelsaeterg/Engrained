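; Projectile actor that flies forward at a set speed and deals damage with knockback to what it strikes, ignoring its instigator.
; On spawn it applies a hue shift to a dynamic material and matches the trail color to it.
; Pawn overlaps and blocking hits send a damage message, spawn hit particles (tinted for overlaps) and destroy it.
; Timelines handle lifetime expiry, stopping the trail and fading opacity before destruction.
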(event `Fire`
  (set `ProjectileMovementComponent.InitialSpeed` 300.0 (`self.ProjectileMovement`)))

(event `SetupDynamicMaterials`
  (bind _returnvalue (`PrimitiveComponent.CreateDynamicMaterialInstance` (`self.ProjectileMesh`) 0 (`PrimitiveComponent.GetMaterial` (`self.ProjectileMesh`) 0) "None"))
  (bind _output_get (set `self.CurrentProjectileDynamicMaterial` _returnvalue))
  (`MaterialInstanceDynamic.SetScalarParameterValue` _output_get "HueShift" (`self.HueShift`))
  (bind _returnvalue_2 (`MaterialInstanceDynamic.K2_GetVectorParameterValue` _output_get "Color"))
  (bind (_h _s _v _a) (`KismetMathLibrary.RGBToHSV` _returnvalue_2))
  (bind _returnvalue_3 (`KismetMathLibrary.HSVToRGB` (+ _h (* (`self.HueShift`) 256.0)) _s _v _a))
  (`FXSystemComponent.SetColorParameter` (`self.ProjectileTrail`) "InColor" _returnvalue_3)
  (set `self.CurrentParticleColor` _returnvalue_3))

(event `self.ProjectileMesh.OnComponentBeginOverlap`
  (params (OverlappedComponent :type "PrimitiveComponent Object Reference") (OtherActor :type "Actor Object Reference") (OtherComp :type "PrimitiveComponent Object Reference") (OtherBodyIndex :type Integer) (bFromSweep :type Boolean) (SweepResult :type "HitResult Structure (by ref)"))
  (bind (_returnvalue_location _returnvalue_rotation _returnvalue_scale) (`KismetMathLibrary.BreakTransform` (`self.GetTransform` self)))
  (`/Engine/EditorBlueprintResources/StandardMacros.IsValid` self
    (:`Is Valid`
      (if (not (== (`self.GetInstigator`) OtherActor))
        (`/Engine/EditorBlueprintResources/StandardMacros.IsValid` self
          (:`Is Valid`
            (if (`|EnumEquality` (`PrimitiveComponent.GetCollisionObjectType` OtherComp) "ECC_Pawn")
              (message `/Game/Blueprints/BPI_CombatInteractionInterface.TakeDamage` OtherActor _returnvalue_location (`KismetMathLibrary.Normal` (`SceneComponent.GetForwardVector` (`self.ProjectileMesh`))) (`self.ProjectileDamage`) (`self.KnockbackPower`))
              (`/Engine/EditorBlueprintResources/StandardMacros.IsValid` self
                (:`Is Valid`
                  (bind _returnvalue (`NiagaraFunctionLibrary.SpawnSystemAtLocation` (`self.OnHitParticles`) _returnvalue_location _returnvalue_rotation _returnvalue_scale true false))
                  (`FXSystemComponent.SetColorParameter` _returnvalue "InColor" (`self.CurrentParticleColor`))
                  (`ActorComponent.Activate` _returnvalue false)
                  (`self.K2_DestroyActor`))))))))))

(event `self.ReceiveBeginPlay`
  (`parent.ReceiveBeginPlay`)
  (`self.SetupDynamicMaterials`)
  (`self.SetNewProjectileSpeed`)
  (`self.StartLifetimer`))

(event `StartLifetimer`
  (bind (_direction _newtrack_0) (`Timeline|Lifetime Timeline`)
    (:`Update`
      (if (< _newtrack_0 0.1)
        (`ActorComponent.Deactivate` (`self.ProjectileTrail`))
        (bind (_direction_2 _newtrack_0_2) (`Timeline|FadeTimeline`)
          (:`Update`
            (`MaterialInstanceDynamic.SetScalarParameterValue` (`self.CurrentProjectileDynamicMaterial`) "Opacity" _newtrack_0_2))
          (:`Finished`
            (`PrimitiveComponent.SetCollisionEnabled` (`self.ProjectileMesh`) "NoCollision")
            (`KismetSystemLibrary.Delay` 0.2)
            (`self.K2_DestroyActor`)))))))

(event `self.ProjectileMesh.OnComponentHit`
  (params (HitComponent :type "PrimitiveComponent Object Reference") (OtherActor :type "Actor Object Reference") (OtherComp :type "PrimitiveComponent Object Reference") (NormalImpulse :type "Vector Structure") (Hit :type "HitResult Structure (by ref)"))
  (bind (_returnvalue_location _returnvalue_rotation _returnvalue_scale) (`KismetMathLibrary.BreakTransform` (`self.GetTransform` self)))
  (`/Engine/EditorBlueprintResources/StandardMacros.IsValid` self
    (:`Is Valid`
      (if (not (== (`self.GetInstigator`) OtherActor))
        (message `/Game/Blueprints/BPI_CombatInteractionInterface.TakeDamage` OtherActor _returnvalue_location (`KismetMathLibrary.Normal` (`SceneComponent.GetForwardVector` (`self.ProjectileMesh`))) (`self.ProjectileDamage`) (`self.KnockbackPower`))
        (`NiagaraFunctionLibrary.SpawnSystemAtLocation` "/Game/Particles/NS_ProjectileHit.NS_ProjectileHit" _returnvalue_location _returnvalue_rotation _returnvalue_scale)
        (`self.K2_DestroyActor`)))))

(event `SetNewProjectileSpeed`
  (set `MovementComponent.Velocity` (* (`SceneComponent.GetForwardVector` (`self.ProjectileMesh`)) (`self.ProjectileSpeed`)) (`self.ProjectileMovement`)))

(fn `UserConstructionScript`)