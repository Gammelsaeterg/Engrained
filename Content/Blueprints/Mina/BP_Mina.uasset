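; BP_Mina is the Blueprint for Mina, an actor that handles pause input and tracks health.
; The Pause Game input lazily creates and caches WBP_PauseMenu, then toggles it along with game pause, mouse cursor and input mode.
; Damage and healing events adjust Health without an upper clamp.
; When damage depletes Health, it sets IsDestroyed on the GameMode and destroys the actor.
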(event `InputAction|Pause Game` :paused true
  (params (Key :type "Key Structure"))
  (bind _returnvalue (`GameplayStatics.GetPlayerController` 0))
  (bind _pause_menu_reference (`self.Pause Menu Reference`))
  ;[1 1 1] Pause and Unpause Game
  (:`Pressed`
    (`/Engine/EditorBlueprintResources/StandardMacros.IsValid` (`self.Pause Menu Reference`)
      (:`Is Valid`
        _)
      (:`Is Not Valid`
        (bind _returnvalue_2 (`|CreateWidget` "/Game/UI/MenusAndSettings/WBP_PauseMenu.WBP_PauseMenu_C"))
        (set `self.Pause Menu Reference` _returnvalue_2)))
    (if (`GameplayStatics.IsGamePaused`)
      (`Widget.RemoveFromParent` _pause_menu_reference)
      (`GameplayStatics.SetGamePaused` false)
      (set `PlayerController.bShowMouseCursor` false _returnvalue)
      (`WidgetBlueprintLibrary.SetInputMode_GameOnly` _returnvalue)
      (else
        (`UserWidget.AddToViewport` _pause_menu_reference 0)
        (`GameplayStatics.SetGamePaused` true)
        (set `PlayerController.bShowMouseCursor` true _returnvalue)
        (`WidgetBlueprintLibrary.SetInputMode_GameAndUIEx` _returnvalue _pause_menu_reference "LockInFullscreen" false)))))

(event `/Game/Blueprints/GameMode/BPI_Damage.Take Damage`
  (params (Damage :type "Float (single-precision)"))
  ;[1 1 1] Taking damage
  (set `self.Health` (- (`self.Health`) Damage))
  ;[1 1 1] If Mina Has less then 0 hp, destroy actor
  (if (<= (`self.Health`) 0.0)
    (set `/Game/Blueprints/GameMode/BP_CrescentGameMode.Is Destroyed` true (`self.GameMode`))
    (`self.K2_DestroyActor`)))

(event `/Game/Blueprints/GameMode/BPI_Healing.Healing`
  (params (Heal :type "Float (single-precision)"))
  ;[1 1 1] Healing Mina
  (set `self.Health` (+ (`self.Health`) Heal)))

(fn `UserConstructionScript`)