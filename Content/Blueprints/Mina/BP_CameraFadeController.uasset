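; BP_CameraFadeController is a component on the player pawn that fades objects standing between the camera and the player.
; Each Tick it multi-line-traces from the camera to the pawn and collects BP_FadeComp components on hit actors.
; It compares its persistent list against a second trace's results, cleared each frame, to restore default materials on components no longer hit.
; Those remaining get their fade material applied.
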(event `self.ReceiveBeginPlay`
  (bind _aspawn (cast `Pawn` (`self.GetOwner`)))
  (bind _output_get (set `self.Player` _aspawn))
  (bind _asplayer_controller (cast `PlayerController` (`Pawn.GetController` _output_get)))
  (set `self.Player Camera Manager` (`PlayerController.PlayerCameraManager` _asplayer_controller)))

(event `self.ReceiveTick`
  (params (DeltaSeconds :type "Float (single-precision)"))
  (bind _player (`self.Player`))
  (bind _player_2 (`self.Player`))
  (set `self.DeltaTime` DeltaSeconds)
  (`|ExecutionSequence`
    (:`then_0`
      (bind _outhits (`KismetSystemLibrary.LineTraceMulti` (`PlayerCameraManager.GetCameraLocation` (`self.Player Camera Manager`)) (`Actor.K2_GetActorLocation` _player) "TraceTypeQuery4" false (`|MakeArray` _player :!type "Actor Object Reference") "None" true (struct :`R` 1.0 :`A` 1.0) (struct :`G` 1.0 :`A` 1.0) (`self.DeltaTime`)))
      (for _array_element _outhits
        (bind _returnvalue (`Actor.GetComponentByClass` (`.HitActor` (`GameplayStatics.BreakHitResult` _array_element)) "/Game/Blueprints/ActorComponents/BP_FadeComp.BP_FadeComp_C"))
        (`/Engine/EditorBlueprintResources/StandardMacros.IsValid` _returnvalue
          (:`Is Valid`
            (`KismetArrayLibrary.Array_AddUnique` (`self.HitActors`) _returnvalue)))))
    (:`then_1`
      (bind _outhits_2 (`KismetSystemLibrary.LineTraceMulti` (`PlayerCameraManager.GetCameraLocation` (`self.Player Camera Manager`)) (`Actor.K2_GetActorLocation` _player_2) "TraceTypeQuery4" false (`|MakeArray` _player_2 :!type "Actor Object Reference") "None" true (struct :`R` 1.0 :`A` 1.0) (struct :`G` 1.0 :`A` 1.0) (`self.DeltaTime`)))
      (for _array_element_2 _outhits_2
        (bind _returnvalue_2 (`Actor.GetComponentByClass` (`.HitActor` (`GameplayStatics.BreakHitResult` _array_element_2)) "/Game/Blueprints/ActorComponents/BP_FadeComp.BP_FadeComp_C"))
        (`/Engine/EditorBlueprintResources/StandardMacros.IsValid` _returnvalue_2
          (:`Is Valid`
            (`KismetArrayLibrary.Array_AddUnique` (`self.HitActors_Comparison`) _returnvalue_2)))))
    (:`then_2`
      (for _array_element_3 (`self.HitActors`)
        (if (== (`KismetArrayLibrary.Array_Find` (`self.HitActors_Comparison`) _array_element_3) -1)
          (`/Game/Blueprints/ActorComponents/BP_FadeComp.Set default materials` _array_element_3)
          (`KismetArrayLibrary.Array_RemoveItem` (`self.HitActors`) _array_element_3))))
    (:`then_3`
      (`KismetArrayLibrary.Array_Clear` (`self.HitActors_Comparison`)))
    (:`then_4`
      (for _array_element_4 (`self.HitActors`)
        (`/Game/Blueprints/ActorComponents/BP_FadeComp.Set Fade Material` _array_element_4)))))