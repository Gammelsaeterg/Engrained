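; Interactable world object that shows written text in an on-screen bubble when the player interacts with it.
; Its overlap zone adds and removes it from the Mina player's interactable list, and it supplies an interaction message.
; The first interaction creates a text bubble widget and starts writing; later ones ask it to continue and return its result.
; Finishing or cancelling removes the widget and resets the interaction.
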(event `BindFinishedInteraction`
  (bind _currentinteractivewiget (`self.CurrentInteractiveWiget`)
    (:`then`
      (add `/Game/UI/InteractiveText/WBP_InteractiveTextBubble.FinishedWriting` _currentinteractivewiget (delegate `Finished`)))
    (:`else`)))

(event `Finished`
  (bind _currentinteractivewiget (`self.CurrentInteractiveWiget`)
    (:`then`
      (`Widget.RemoveFromParent` _currentinteractivewiget :!label _label))
    (:`else`
      _))
  (set `self.bInteractionStarted` false))

(event `/Game/Blueprints/BP_PlayerInteractionInterface.CancelInteraction`
  (goto _label))

(event `self.InteractiveZone.OnComponentBeginOverlap`
  (params (OverlappedComponent :type "PrimitiveComponent Object Reference") (OtherActor :type "Actor Object Reference") (OtherComp :type "PrimitiveComponent Object Reference") (OtherBodyIndex :type Integer) (bFromSweep :type Boolean) (SweepResult :type "HitResult Structure (by ref)"))
  ;[1 1 1] Player overlap
  (bind _asbp_mina_prototype_blueprint_only (cast `/Game/Blueprints/BP_MinaPrototypeBlueprintOnly` OtherActor))
  (`/Game/Blueprints/BP_MinaPrototypeBlueprintOnly.AddInteractableToList` _asbp_mina_prototype_blueprint_only self))

(event `self.InteractiveZone.OnComponentEndOverlap`
  (params (OverlappedComponent :type "PrimitiveComponent Object Reference") (OtherActor :type "Actor Object Reference") (OtherComp :type "PrimitiveComponent Object Reference") (OtherBodyIndex :type Integer))
  ;[1 1 1] Player overlap
  (bind _asbp_mina_prototype_blueprint_only (cast `/Game/Blueprints/BP_MinaPrototypeBlueprintOnly` OtherActor))
  (`/Game/Blueprints/BP_MinaPrototypeBlueprintOnly.RemoveInteractableFromList` _asbp_mina_prototype_blueprint_only self))

(fn `GetInteractionMessage`
  (returns (GetInteractionMessage :type String))
  (return (`self.PlayerInteractionMessage`)))

(fn `PlayerInteract`
  (params (PlayerInteracting :type "PlayerController Object Reference"))
  (returns (InteractionComplete :type Boolean))
  (bind _currentinteractivewiget (`self.CurrentInteractiveWiget`))
  (if (not (`self.bInteractionStarted`))
    (set `self.bInteractionStarted` true)
    (bind _returnvalue (`|CreateWidget` "/Game/UI/InteractiveText/WBP_InteractiveTextBubble.WBP_InteractiveTextBubble_C" PlayerInteracting (`self.TextToWrite`) (`self.DefaultWordsPerSecond`)))
    (bind _output_get (set `self.CurrentInteractiveWiget` _returnvalue))
    (`/Game/UI/InteractiveText/WBP_InteractiveTextBubble.Write` _output_get)
    (`self.BindFinishedInteraction`)
    (`UserWidget.AddToViewport` _returnvalue 0)
    (return false)
    (else
      (`/Engine/EditorBlueprintResources/StandardMacros.IsValid` _currentinteractivewiget
        (:`Is Valid`
          (bind _binteractionfinished (`/Game/UI/InteractiveText/WBP_InteractiveTextBubble.ContinueText` _currentinteractivewiget))
          (return _binteractionfinished))))))

(fn `UserConstructionScript`)