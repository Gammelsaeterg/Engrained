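; Whaleshroom actor that travels along a referenced spline from BeginPlay, with configurable duration and start offset.
; The Whalemover timeline's alpha maps to distance along the spline, setting location and, when Rotation is enabled, the spline's rotation.
; With Rotation off, Tick compares height against the previous frame and eases pitch between negative and positive TiltAngle as it descends or climbs.
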(event `MoveWhale`
  (bind _spline (`/Game/Blueprints/Whaleshroom/BP_Spline.Spline` (`self.Spline`)))
  (bind _spline_2 (`/Game/Blueprints/Whaleshroom/BP_Spline.Spline` (`self.Spline`)))
  (bind _returnvalue (`KismetMathLibrary.Lerp` 0.0 (`SplineComponent.GetSplineLength` _spline_2) (`self.Alpha`)))
  (`TimelineComponent.SetPlayRate` (`self.Whalemover`) (/ 1.0 (`self.Duration`)))
  (`TimelineComponent.SetNewTime` (`self.Whalemover`) (`self.Start Offset`))
  (bind (_direction _alpha) (`Timeline|Whalemover`)
    (:`Update`
      (set `self.Alpha` _alpha)
      (if (`self.bRotation`)
        (`self.K2_SetActorLocationAndRotation` (`SplineComponent.GetLocationAtDistanceAlongSpline` _spline_2 _returnvalue "World") (`SplineComponent.GetRotationAtDistanceAlongSpline` (`/Game/Blueprints/Whaleshroom/BP_Spline.Spline` (`self.Spline`)) _returnvalue "World"))
        (else
          (`self.K2_SetActorLocation` (`SplineComponent.GetLocationAtDistanceAlongSpline` _spline (`KismetMathLibrary.Lerp` 0.0 (`SplineComponent.GetSplineLength` _spline) (`self.Alpha`)) "World")))))))

(event `self.ReceiveBeginPlay`
  (`self.MoveWhale`))

(event `self.ReceiveTick`
  (params (DeltaSeconds :type "Float (single-precision)"))
  (bind _z (.z (- (`self.Current Location`) (`self.Last Location`))))
  (set `self.Delta Seconds` DeltaSeconds)
  (if (not (`self.bRotation`))
    (set `self.Current Location` (`self.K2_GetActorLocation`))
    (`|ExecutionSequence`
      (:`then_0`
        (if (> _z 0.0)
          (if (>= (`self.PitchAlpha`) 1.0)
            (set `self.PitchAlpha` 1.0)
            (else
              (set `self.PitchAlpha` (+ (`self.PitchAlpha`) (`self.Delta Seconds`)))))
          (`self.K2_SetActorRotation` (`KismetMathLibrary.MakeRotator` 0.0 (`KismetMathLibrary.Lerp` (* (`self.TiltAngle`) -1.0) (`self.TiltAngle`) (`self.PitchAlpha`))) :!label _label)
          (elif (< _z 0.0)
            (if (<= (`self.PitchAlpha`) 0.0)
              (set `self.PitchAlpha` 0.0)
              (goto _label)
              (else
                (set `self.PitchAlpha` (- (`self.PitchAlpha`) (`self.Delta Seconds`)))
                (goto _label))))))
      (:`then_1`
        (set `self.Last Location` (`self.Current Location`))))))

(fn `UserConstructionScript`)