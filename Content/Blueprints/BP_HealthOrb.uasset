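; Health orb pickup that scatters on spawn, then homes in on the MinaExperimental player to grant health.
; BeginPlay randomizes scale and drift, while timelines drive emissive glow and launch motion, enabling collision after a short delay.
; After a timer, Tick moves it toward the player's Neck socket by the remaining offset divided by a timeline-driven Speed.
; Player overlap sends HealthAmount, hides the orb, plays particles and sound, then destroys it.
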(event `self.ReceiveBeginPlay`
  (bind _returnvalue (`KismetMathLibrary.RandomFloatInRange` 0.1 0.2))
  (bind _returnvalue_2 (`KismetMathLibrary.RandomFloatInRange` -2.0 2.0))
  (`PrimitiveComponent.SetCollisionEnabled` (`self.Sphere`) "NoCollision")
  (`self.SetActorScale3D` (`KismetMathLibrary.MakeVector` _returnvalue _returnvalue _returnvalue))
  (set `self.Initial_Force_X` _returnvalue_2)
  (set `self.Initial_Force_Y` _returnvalue_2)
  (bind _asmina_experimental (cast `MinaExperimental` (`GameplayStatics.GetPlayerPawn` 0)))
  (set `self.As Mina Experimental` _asmina_experimental)
  (`KismetSystemLibrary.K2_SetTimerDelegate` (delegate `MoveToPlayer`) 2.0)
  (bind (_direction _newtrack_0) (`Timeline|Material Emissive Strength`)
    (:`Update`
      (`MeshComponent.SetScalarParameterValueOnMaterials` (`self.Sphere`) "EmissiveStrength" _newtrack_0)
      (bind (_direction_2 _newtrack_0_2) (`Timeline|Initial Force`)
        (:`Update`
          (bind _output_get (set `self.Initial_Force` _newtrack_0_2))
          (`SceneComponent.K2_AddRelativeLocation` (`self.DefaultSceneRoot`) (`KismetMathLibrary.MakeVector` (`self.Initial_Force_X`) (`self.Initial_Force_Y`) _output_get) false false)
          (`KismetSystemLibrary.Delay` 0.3)
          (`PrimitiveComponent.SetCollisionEnabled` (`self.Sphere`) "QueryAndPhysics"))))))

(event `MoveToPlayer`
  (set `self.bMovingToPlayer` true)
  (bind (_direction _speed) (`Timeline|Speed Timeline`)
    (:`Update`
      (set `self.Speed` _speed))))

(event `self.Sphere.OnComponentBeginOverlap`
  (params (OverlappedComponent :type "PrimitiveComponent Object Reference") (OtherActor :type "Actor Object Reference") (OtherComp :type "PrimitiveComponent Object Reference") (OtherBodyIndex :type Integer) (bFromSweep :type Boolean) (SweepResult :type "HitResult Structure (by ref)"))
  (bind _sphere (`self.Sphere`))
  (if (== OtherActor (`self.As Mina Experimental`))
    (set `self.bMovingToPlayer` false)
    (message `/Game/Blueprints/BPI_CombatInteractionInterface.GetHealth` OtherActor (`self.HealthAmount`))
    (`SceneComponent.SetVisibility` _sphere false false)
    (`PrimitiveComponent.SetCollisionEnabled` _sphere "NoCollision")
    (`ActorComponent.Activate` (`self.ParticleOnDestroy`) false)
    (`GameplayStatics.SpawnSoundAtLocation` "/Game/Sounds/CreativeCommons/FOOTSTEP3_504479__joao-janz__rock-hitting-log-1-5.FOOTSTEP3_504479__joao-janz__rock-hitting-log-1-5" (`self.K2_GetActorLocation`) (struct) 1.0 1.0 0.0 "/Game/Sounds/SA_CaveSoundAttenuation.SA_CaveSoundAttenuation" null)
    (`KismetSystemLibrary.Delay` 1.0)
    (`self.K2_DestroyActor`)))

(event `self.ReceiveTick`
  (params (DeltaSeconds :type "Float (single-precision)"))
  (bind _initial_force_y (`self.Initial_Force_Y`))
  (bind _initial_force_x (`self.Initial_Force_X`))
  (if (> _initial_force_x 0.0)
    (set `self.Initial_Force_X` (- _initial_force_x DeltaSeconds))
    (else
      (set `self.Initial_Force_X` (+ _initial_force_x DeltaSeconds))))
  (if (> _initial_force_y 0.0)
    (set `self.Initial_Force_Y` (- _initial_force_y DeltaSeconds))
    (else
      (set `self.Initial_Force_Y` (+ _initial_force_y DeltaSeconds))))
  (if (`self.bMovingToPlayer`)
    (`SceneComponent.K2_AddRelativeLocation` (`self.DefaultSceneRoot`) (/ (- (`SceneComponent.GetSocketLocation` (`Actor.RootComponent` (`self.As Mina Experimental`)) "Neck") (`self.K2_GetActorLocation`)) (`self.Speed`)) false false)))

(fn `UserConstructionScript`)