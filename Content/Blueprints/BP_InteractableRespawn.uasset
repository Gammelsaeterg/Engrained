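; Interactable respawn point that saves a new checkpoint for the Mina player character and glows to show it is the active one.
; Its interaction box adds it to the player's interactable list on capsule overlap, unless already activated.
; Interacting passes the RespawnLocation transform to the player, then deactivates any other active point of the same class.
; Timelines fade a dynamic material's emissive strength in or out while toggling spore effects.
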(event `self.InteractionBox.OnComponentBeginOverlap`
  (params (OverlappedComponent :type "PrimitiveComponent Object Reference") (OtherActor :type "Actor Object Reference") (OtherComp :type "PrimitiveComponent Object Reference") (OtherBodyIndex :type Integer) (bFromSweep :type Boolean) (SweepResult :type "HitResult Structure (by ref)"))
  ;[1 1 1] Player interaction setup
  (bind _asbp_mina_prototype_blueprint_only (cast `/Game/Blueprints/Mina/BP_MinaPrototypeBlueprintOnly` OtherActor))
  (if (== (`GameplayStatics.GetObjectClass` OtherComp) "/Script/Engine.CapsuleComponent")
    (if (not (`self.bIsActivated`))
      (`/Game/Blueprints/Mina/BP_MinaPrototypeBlueprintOnly.AddInteractableToList` _asbp_mina_prototype_blueprint_only self))))

(event `self.InteractionBox.OnComponentEndOverlap`
  (params (OverlappedComponent :type "PrimitiveComponent Object Reference") (OtherActor :type "Actor Object Reference") (OtherComp :type "PrimitiveComponent Object Reference") (OtherBodyIndex :type Integer))
  ;[1 1 1] Player interaction setup
  (bind _asbp_mina_prototype_blueprint_only (cast `/Game/Blueprints/Mina/BP_MinaPrototypeBlueprintOnly` OtherActor))
  (if (== (`GameplayStatics.GetObjectClass` OtherComp) "/Script/Engine.CapsuleComponent")
    (`/Game/Blueprints/Mina/BP_MinaPrototypeBlueprintOnly.RemoveInteractableFromList` _asbp_mina_prototype_blueprint_only self)))

(event `self.ReceiveBeginPlay`
  (bind _spawnmesh (`self.SpawnMesh`))
  (bind _returnvalue (`PrimitiveComponent.CreateDynamicMaterialInstance` _spawnmesh 0 (`|GetArrayItem` (`MeshComponent.GetMaterials` _spawnmesh) 2) "None"))
  (bind _output_get (set `self.DynamicMaterialInstance` _returnvalue))
  (set `self.CurrentDynamicMaterial` _output_get))

(event `ActivateRespawn`
  (bind _outactors (`GameplayStatics.GetAllActorsOfClass` (`GameplayStatics.GetObjectClass` self)))
  (for _array_element _outactors
    (if (`/Game/Blueprints/BP_InteractableRespawn.bIsActivated` _array_element)
      (`self.DeactivateRespawn` _array_element)))
  (set `self.bIsActivated` true)
  (bind (_direction _glowcurve) (`Timeline|GlowTimeline` :!via `PlayFromStart`)
    (:`Update`
      (bind _currentdynamicmaterial (`self.CurrentDynamicMaterial`)
        (:`then`
          (`MaterialInstanceDynamic.SetScalarParameterValue` _currentdynamicmaterial "EmissiveStrength" (* _glowcurve 3.0))
          (`ActorComponent.Activate` (`self.Spores`) true))
        (:`else`)))))

(event `DeactivateRespawn`
  (set `self.bIsActivated` false)
  (bind (_direction _glowcurve) (`Timeline|GlowTimelineReverse` :!via `ReverseFromEnd`)
    (:`Update`
      (bind _currentdynamicmaterial (`self.CurrentDynamicMaterial`)
        (:`then`
          (`MaterialInstanceDynamic.SetScalarParameterValue` _currentdynamicmaterial "EmissiveStrength" (* _glowcurve 3.0))
          (`ActorComponent.Deactivate` (`self.Spores`)))
        (:`else`)))))

(fn `GetInteractionMessage`
  (returns (GetInteractionMessage :type String))
  (return (`self.PlayerInteractionMessage`)))

(fn `PlayerInteract`
  (params (PlayerInteracting :type "PlayerController Object Reference"))
  (returns (InteractionComplete :type Boolean))
  (bind _asbp_mina_prototype_blueprint_only (cast `/Game/Blueprints/Mina/BP_MinaPrototypeBlueprintOnly` (`Controller.K2_GetPawn` PlayerInteracting)))
  (`/Game/Blueprints/Mina/BP_MinaPrototypeBlueprintOnly.SaveNewCheckpoint` _asbp_mina_prototype_blueprint_only (`SceneComponent.K2_GetComponentToWorld` (`self.RespawnLocation`)))
  (`self.ActivateRespawn`)
  (return false))

(fn `UserConstructionScript`)