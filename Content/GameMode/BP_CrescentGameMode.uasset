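; BP_CrescentGameMode is a game mode that handles respawning of the Mina_BP player character.
; BeginPlay and the Respawn event bind OnDestroyed to the current character's destruction, though that handler is empty.
; Tick polls IsDestroyed, waits briefly, spawns a new Mina_BP at SpawnTransform, possesses it, rebinds and clears the flag.
; Nothing in this graph sets IsDestroyed to true.
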(event `Respawn`
  ;[1 1 1] Respawn System
  (bind _asmina_bp (cast `/Game/MinaBody/Mina_BP` (`GameplayStatics.GetPlayerCharacter` 0) :!label _label))
  (if true
    (add `Actor.OnDestroyed` _asmina_bp (delegate `On Destroyed`))))

(event `self.ReceiveBeginPlay`
  ;[1 1 1] Respawn System
  (goto _label))

(event `On Destroyed`
  (params (DestroyedActor :type "Actor Object Reference"))
  ;[1 1 1] Respawn System
)

(event `self.ReceiveTick`
  (params (DeltaSeconds :type "Float (single-precision)"))
  ;[1 1 1] Respawn System
  (if (`self.Is Destroyed`)
    (`KismetSystemLibrary.Delay` 1.0)
    (bind _returnvalue (`|SpawnActorFromClass` "/Game/MinaBody/Mina_BP.Mina_BP_C" (`self.Spawn Transform`) "Undefined" "OverrideRootScale" null null))
    (`Controller.Possess` (`GameplayStatics.GetPlayerController` 0) _returnvalue)
    (`self.Respawn`)
    (set `self.Is Destroyed` false)))

(fn `UserConstructionScript`)